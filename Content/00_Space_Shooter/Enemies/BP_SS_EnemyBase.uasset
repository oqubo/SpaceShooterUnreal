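; Base enemy actor for a space shooter that flies straight ahead and fires automatically.
; Tick moves it along the forward vector cached at BeginPlay and spawns Ammo at FirePoint, matching its rotation, whenever the shot timer exceeds DelayShoot.
; Overlapping a Player-tagged actor calls the OnEnemyDestroy dispatcher and notifies SS_GameMode.
; Its own handler bound to that dispatcher destroys the actor after a short delay.
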(event `self.ReceiveBeginPlay`
  ; Movimiento hacia adelante
  (set `self.MovementVector` (`self.GetActorForwardVector`))
  ; Escucha si lo destruyen
  (add `self.OnEnemyDestroy` (delegate `Destroyed_Event`)))

(event `Destroyed_Event`
  ; Escucha si lo destruyen
  (`KismetSystemLibrary.Delay` 0.1)
  (`self.K2_DestroyActor`))

(event `self.ReceiveActorBeginOverlap`
  (params (OtherActor :type "Actor Object Reference"))
  ; Si colisiona con la nave o disparo del player (tag) llamamos a enemy destroyed (del game mode)
  (if (`KismetArrayLibrary.Array_Contains` (`Actor.Tags` OtherActor) "Player")
    (`self.OnEnemyDestroy`)
    (bind _asss_game_mode (cast `/Game/00_Space_Shooter/SS_GameMode` (`GameplayStatics.GetGameMode`)))
    (`/Game/00_Space_Shooter/SS_GameMode.Enemy Destroyed` _asss_game_mode)))

(event `self.ReceiveTick`
  (params (DeltaSeconds :type "Float (single-precision)"))
  ; En cada fotograma movemos y disparamos de forma automática
  (`self.Move` DeltaSeconds)
  (bind _output_get (set `self.ShotCurrentTime` (+ DeltaSeconds (`self.ShotCurrentTime`))))
  (if (> _output_get (`self.DelayShoot`))
    (set `self.ShotCurrentTime` 0.0)
    (`self.Fire`)))

(fn `Fire`
  (bind _returnvalue (`|SpawnActorFromClass` (`self.Ammo`) (`SceneComponent.K2_GetComponentToWorld` (`self.FirePoint`)) "Undefined" "MultiplyWithRoot" null null))
  (`self.K2_SetActorRotation` _returnvalue (`self.K2_GetActorRotation`) false))

(fn `Move`
  (params (`Delta Time` :type "Float (double-precision)"))
  (`self.K2_SetActorLocation` (+ (`self.K2_GetActorLocation`) (* (* `Delta Time` (`self.Speed`)) (`self.MovementVector`)))))

(fn `UserConstructionScript`)