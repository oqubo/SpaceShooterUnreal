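; Space shooter enemy Blueprint that sets a horizontal movement direction and reverses it at lateral boundaries.
; It starts along its right vector, then flips MovementVector whenever it overlaps an actor tagged "Lateral".
; Each switch from right to left also shortens DelayShoot, with no lower clamp here.
; BeginPlay and overlap call the parent first; this graph only sets values, without moving or shooting itself.
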(event `self.ReceiveBeginPlay`
  (`parent.ReceiveBeginPlay`)
  (set `self.MovementVector` (`self.GetActorRightVector`))
  (set `self.isRight` true))

(event `self.ReceiveActorBeginOverlap`
  (params (OtherActor :type "Actor Object Reference"))
  (bind _returnvalue (`self.GetActorRightVector`))
  (`parent.ReceiveActorBeginOverlap` OtherActor)
  (if (`KismetArrayLibrary.Array_Contains` (`Actor.Tags` OtherActor) "Lateral")
    (if (`self.isRight`)
      (set `self.isRight` false)
      (set `self.MovementVector` (* _returnvalue -1.0))
      (set `self.DelayShoot` (- (`self.DelayShoot`) 0.1))
      (else
        (set `self.isRight` true)
        (set `self.MovementVector` _returnvalue)))))

(fn `UserConstructionScript`
  (`parent.UserConstructionScript`))