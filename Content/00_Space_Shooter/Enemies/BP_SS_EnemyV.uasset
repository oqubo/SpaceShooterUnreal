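; BP_SS_EnemyV is a space shooter enemy that moves and fires from two points at a regular interval.
; Each Tick calls Move, which is defined outside this graph, and accumulates a shot timer.
; When the timer exceeds DelayShoot, it resets and Fire2 spawns the Ammo class at the transforms of FirePoint and FirePoint1.
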(event `self.ReceiveTick`
  (params (DeltaSeconds :type "Float (single-precision)"))
  (`self.Move` DeltaSeconds)
  (bind _output_get (set `self.ShotCurrentTime` (+ DeltaSeconds (`self.ShotCurrentTime`))))
  (if (> _output_get (`self.DelayShoot`))
    (set `self.ShotCurrentTime` 0.0)
    (`self.Fire2` (`SceneComponent.K2_GetComponentToWorld` (`self.FirePoint`)))
    (`self.Fire2` (`SceneComponent.K2_GetComponentToWorld` (`self.FirePoint1`)))))

(fn `Fire2`
  (params (FirePoint :type "Transform Structure"))
  (`|SpawnActorFromClass` (`self.Ammo`) FirePoint "Undefined" "MultiplyWithRoot" null null))

(fn `UserConstructionScript`
  (`parent.UserConstructionScript`))