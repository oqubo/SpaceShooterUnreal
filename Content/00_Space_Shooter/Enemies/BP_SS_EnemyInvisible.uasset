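; Space shooter enemy Blueprint that flickers in and out of visibility during play.
; Each Tick runs the parent logic, applies the Hidden flag through SetActorHiddenInGame, then uses chained Delays to set the flag and later clear it.
; The Delays sit directly on Tick, so the first re-arms while the second is pending and their cycles overlap rather than alternate cleanly.
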(event `self.ReceiveTick`
  (params (DeltaSeconds :type "Float (single-precision)"))
  (`parent.ReceiveTick` DeltaSeconds)
  (`self.SetActorHiddenInGame` (`self.hidden`))
  (`KismetSystemLibrary.Delay` 1.0)
  (bind _output_get (set `self.hidden` true))
  (`self.SetActorHiddenInGame` _output_get)
  (`KismetSystemLibrary.Delay` 2.0)
  (set `self.hidden` false))

(fn `UserConstructionScript`
  (`parent.UserConstructionScript`))