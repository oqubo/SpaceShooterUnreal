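; Three-shot power-up pickup actor for the space shooter, named for the effect but containing no logic that grants it.
; Tick moves it along its forward vector by Speed scaled with delta time, without sweeping.
; On overlap with an actor tagged Player it destroys itself, passing nothing to that actor.
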(event `self.ReceiveActorBeginOverlap`
  (params (OtherActor :type "Actor Object Reference"))
  (if (`KismetArrayLibrary.Array_Contains` (`Actor.Tags` OtherActor) "Player")
    (`self.K2_DestroyActor`)))

(event `self.ReceiveTick`
  (params (DeltaSeconds :type "Float (single-precision)"))
  (`self.K2_SetActorLocation` (+ (`self.K2_GetActorLocation`) (* (* DeltaSeconds (`self.speed`)) (`self.GetActorForwardVector`)))))

(fn `UserConstructionScript`)