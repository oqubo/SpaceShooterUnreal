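; Power-up generator actor for the space shooter that periodically spawns pickups at random spawn points.
; On BeginPlay it caches the game mode and starts a looping timer on SpawnTime.
; Each tick of that timer spawns a triple-shot or shot-delay power-up at a random component tagged SpawnPoint.
; SpawnPowerUp and GetClassToSpawn, unused by the timer, instead pick enemy classes by game level, apparently left over from an enemy spawner.
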(event `self.ReceiveBeginPlay`
  (bind _asss_game_mode (cast `/Game/00_Space_Shooter/SS_GameMode` (`GameplayStatics.GetGameMode`)))
  (set `self.m_GameMode` _asss_game_mode)
  (`KismetSystemLibrary.K2_SetTimerDelegate` (delegate `Spwan`) (`self.spawnTime`) true))

(event `Spwan`
  (bind _returnvalue (`self.GetComponentsByTag` "/Script/Engine.ActorComponent" "SpawnPoint"))
  ; Selecciono el punto de spawn
  (bind _asscene_component (cast `SceneComponent` (`|GetArrayItem` _returnvalue (`KismetMathLibrary.RandomInteger` (`KismetArrayLibrary.Array_Length` _returnvalue)))))
  (`|SpawnActorFromClass` (select `int` (`KismetMathLibrary.RandomInteger` 2) :`0` "/Game/00_Space_Shooter/PowerUp/BP_SS_PowerUp3Shot.BP_SS_PowerUp3Shot_C" :`1` "/Game/00_Space_Shooter/PowerUp/BP_SS_PowerUpShotDelay.BP_SS_PowerUpShotDelay_C" :!type "Actor Class Reference") (`SceneComponent.K2_GetComponentToWorld` _asscene_component) "Undefined" "MultiplyWithRoot" null null))

(fn `GetClassToSpawn`
  (params (type :type Integer))
  (returns (Class :type "/Game/00_Space_Shooter/Enemies/BP_SS_EnemyBase Class Reference"))
  (return (select `int` (`KismetMathLibrary.Clamp` type 0 (- (`self.maxNumEnemmies`) 1)) :`0` "/Game/00_Space_Shooter/Enemies/BP_SS_EnemyBase.BP_SS_EnemyBase_C" :`1` "/Game/00_Space_Shooter/Enemies/BP_SS_EnemyH.BP_SS_EnemyH_C" :`2` "/Game/00_Space_Shooter/Enemies/BP_SS_EnemyV.BP_SS_EnemyV_C" :`3` "/Game/00_Space_Shooter/Enemies/BP_SS_EnemyInvisible.BP_SS_EnemyInvisible_C" :!type "/Game/00_Space_Shooter/Enemies/BP_SS_EnemyBase Class Reference")))

(fn `SpawnPowerUp`
  (returns (Spawned :type "/Game/00_Space_Shooter/Enemies/BP_SS_EnemyBase Object Reference"))
  (bind _returnvalue (`self.GetComponentsByTag` "/Script/Engine.ActorComponent" "SpawnPoint"))
  (bind _class (`self.GetClassToSpawn` (`KismetMathLibrary.RandomInteger` (`/Game/00_Space_Shooter/SS_GameMode.level` (`self.m_GameMode`)))))
  (bind _asscene_component (cast `SceneComponent` (`|GetArrayItem` _returnvalue (`KismetMathLibrary.RandomInteger` (`KismetArrayLibrary.Array_Length` _returnvalue)))))
  (bind _returnvalue_2 (`|SpawnActorFromClass` _class (`SceneComponent.K2_GetComponentToWorld` _asscene_component) "Undefined" "MultiplyWithRoot" null null))
  (return _returnvalue_2))

(fn `UserConstructionScript`)