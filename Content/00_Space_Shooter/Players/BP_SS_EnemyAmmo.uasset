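; BP_SS_EnemyAmmo is an enemy projectile actor for the space shooter.
; Each tick it moves along its forward vector at Speed, scaled by delta time, without sweeping.
; On any actor overlap it spawns an explosion emitter, plays a 2D explosion sound, waits briefly and destroys itself, with no filtering or damage logic.
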(event `self.ReceiveActorBeginOverlap`
  (params (OtherActor :type "Actor Object Reference"))
  ; Si choca generamos explosion, sonido, delay y se destruye
  (`GameplayStatics.SpawnEmitterAtLocation` "/Game/StarterContent/Particles/P_Explosion.P_Explosion" (`self.K2_GetActorLocation`))
  (`GameplayStatics.PlaySound2D` "/Game/StarterContent/Audio/Explosion02.Explosion02" 1.0 1.0 0.0 null null)
  (`KismetSystemLibrary.Delay` 0.2)
  (`self.K2_DestroyActor`))

(event `self.ReceiveTick`
  (params (DeltaSeconds :type "Float (single-precision)"))
  ; Mover hacia adelante con la velocidad speed
  (`self.K2_SetActorLocation` (+ (`self.K2_GetActorLocation`) (* (`self.GetActorForwardVector`) (* DeltaSeconds (`self.speed`))))))

(fn `UserConstructionScript`)