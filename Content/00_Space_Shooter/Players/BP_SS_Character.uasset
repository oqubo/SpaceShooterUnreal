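; Player character for the space shooter, handling movement, shooting and lives.
; BeginPlay adds the Enhanced Input mapping context, and input actions drive movement along the actor's axes and trigger fire.
; DoFire spawns ammo at the central cannon, with a timer enforcing the delay between shots.
; Overlapping an Enemy-tagged actor removes a life through DamageActor, which calls PlayerDead on the GameMode when lives reach zero.
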(event `self.ReceiveBeginPlay`
  ; Inicializar las entradas del usuario (mapping context)
  (bind _asplayer_controller (cast `PlayerController` (`self.GetController`)))
  (bind _returnvalue (pcsubsystem `EnhancedInputLocalPlayerSubsystem` _asplayer_controller))
  (`/Engine/EditorBlueprintResources/StandardMacros.IsValid` _returnvalue
    (:`Is Valid`
      (`EnhancedInputSubsystemInterface.AddMappingContext` _returnvalue "/Game/00_Space_Shooter/Input/IMC_Player.IMC_Player" 0 (struct)))))

(event `self.ReceiveActorBeginOverlap`
  (params (OtherActor :type "Actor Object Reference"))
  ; Colision con enemigo o disparo (tag Enemy) llama a Damage Actor
  (if (`KismetArrayLibrary.Array_Contains` (`Actor.Tags` OtherActor) "Enemy")
    (bind _asbp_ss_character (cast `/Game/00_Space_Shooter/Players/BP_SS_Character` (`GameplayStatics.GetPlayerPawn` 0)))
    (`self.DamageActor` _asbp_ss_character)))

(event `EnhancedInput|/Game/00_Space_Shooter/Input/IA_Player_Movement`
  (params (ActionValue :type "Vector2D Structure") (ElapsedSeconds :type "Float (double-precision)") (TriggeredSeconds :type "Float (double-precision)") (InputAction :type "InputAction Object Reference" :default "/Game/00_Space_Shooter/Input/IA_Player_Movement.IA_Player_Movement"))
  ; InputAction Movement
  (:`Triggered`
    (`self.AddMovementInput` (`self.GetActorRightVector`) ActionValue_X)
    (`self.AddMovementInput` (`self.GetActorForwardVector`) ActionValue_Y)))

(event `EnhancedInput|/Game/00_Space_Shooter/Input/IA_Player_Fire`
  (params (ActionValue :type Boolean) (ElapsedSeconds :type "Float (double-precision)") (TriggeredSeconds :type "Float (double-precision)") (InputAction :type "InputAction Object Reference" :default "/Game/00_Space_Shooter/Input/IA_Player_Fire.IA_Player_Fire"))
  ; InputAction Fire
  (:`Triggered`
    (if (`self.CanFire`)
      (`self.DoFire`)
      (set `self.CanFire` false)
      (`KismetSystemLibrary.K2_SetTimerDelegate` (delegate `EventFireDelay`) (`self.FireDelay`)))))

(event `EventFireDelay`
  ; InputAction Fire
  (set `self.CanFire` true))

(event `DamageActor`
  ; Damage Actor (le quita 1 vida y si es 0 lo mata, llamando a funcion en GameMode de game over)
  (bind _output_get (set `self.Lifes` (- (`self.Lifes`) 1)))
  (if (== _output_get 0)
    (bind _asss_game_mode (cast `/Game/00_Space_Shooter/SS_GameMode` (`GameplayStatics.GetGameMode`)))
    (`/Game/00_Space_Shooter/SS_GameMode.PlayerDead` _asss_game_mode)))

(fn `DoFire`
  (bind _returnvalue (`|SpawnActorFromClass` "/Game/00_Space_Shooter/Players/BP_SS_Ammo.BP_SS_Ammo_C" (`KismetMathLibrary.Conv_VectorToTransform` (`SceneComponent.K2_GetComponentLocation` (`self.PointCannonCentral`))) "Undefined" "MultiplyWithRoot" null null))
  (`self.K2_SetActorRotation` _returnvalue (struct :`Yaw` 90.0) false))

(fn `UserConstructionScript`)